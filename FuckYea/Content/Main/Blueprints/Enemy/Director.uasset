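; Wave director actor that spawns enemies in rounds and reports the current round to the main UI widget.
; Tick uses Delay nodes to pace random picks from EnemyClasses, spawned near the director with random X offset until the round's limit is reached.
; Health and Damage scale from class defaults by round number.
; Bound death events decrement the alive count; at zero, a rest period precedes a larger next round.
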(event `self.ReceiveBeginPlay`
  (bind _foundwidgets (`WidgetBlueprintLibrary.GetAllWidgetsOfClass` "/Game/Main/Blueprints/UI/W_MainUI.W_MainUI_C"))
  (set `self.MainUI` (`KismetArrayLibrary.Array_Get` _foundwidgets)))

(event `self.ReceiveTick`
  (params (DeltaSeconds :type "Float (single-precision)"))
  (bind _resttime (`self.RestTime`))
  (bind _item (`KismetArrayLibrary.Array_Get` (`self.EnemyClasses`) (`KismetMathLibrary.RandomIntegerInRange` 0 (- (`KismetArrayLibrary.Array_Length` (`self.EnemyClasses`)) 1))))
  (bind (_health _damage) (defaults `/Game/Main/Blueprints/Enemy/Director` _item))
  (if (`self.RestPeriod`)
    ;[1 1 1] TODO : Initial rest period
    (`KismetSystemLibrary.Delay` 3.0)
    (set `self.RestPeriod` false)
    (else
      ;[1 1 1] Make sure the Rest period only starts when the enemy's are daed
      (if (<= (`self.AliveEnemys`) 0)
        (set `self.RestPeriod` true)
        (`KismetSystemLibrary.PrintString` "Rest period" true true (struct :`G` 0.66 :`B` 1.0 :`A` 1.0) _resttime)
        (`KismetSystemLibrary.Delay` _resttime)
        (set `self.RestPeriod` false)
        (bind _output_get (set `self.SpawnLimit` (+ (`self.SpawnLimit`) 5)))
        (set `self.AliveEnemys` _output_get)
        (set `self.SpawnedEnemys` 0)
        (bind _result (`/Engine/EditorBlueprintResources/StandardMacros.IncrementInt` (`self.CurrentRound`))
          (:`  `
            (`/Game/Main/Blueprints/UI/W_MainUI.SetRound` (`self.MainUI`) _result)))
        (elif (not (>= (`self.SpawnedEnemys`) (`self.SpawnLimit`)))
          (`KismetSystemLibrary.Delay` (`self.SpawnRate`))
          (bind _returnvalue (`|SpawnActorFromClass` _item (`KismetMathLibrary.MakeTransform` (+ (`self.K2_GetActorLocation`) (`KismetMathLibrary.MakeVector` (* (`KismetMathLibrary.RandomFloat`) (`self.RandSpawnModifier`)))) (`self.K2_GetActorRotation`)) "Undefined" "OverrideRootScale" null (+ _health (* (/ _health 3.0) (`KismetMathLibrary.Conv_IntToDouble` (`self.CurrentRound`)))) (+ _damage (* (/ _damage 2.0) (`KismetMathLibrary.Conv_IntToDouble` (`self.CurrentRound`))))))
          (`/Engine/EditorBlueprintResources/StandardMacros.IsValid` _returnvalue
            (:`Is Valid`
              (add `/Game/Main/Blueprints/Enemy/BP_ParentEnemy.EnemyAmountDecrease` _returnvalue (delegate `EnemyDied`))
              (`/Engine/EditorBlueprintResources/StandardMacros.IncrementInt` (`self.SpawnedEnemys`)))
            (:`Is Not Valid`
              (`KismetSystemLibrary.PrintString` "Not Valid"))))))))

(event `EnemyDied`
  (bind _result (`/Engine/EditorBlueprintResources/StandardMacros.DecrementInt` (`self.AliveEnemys`))
    (:`  `
      (`KismetSystemLibrary.PrintString` (`KismetStringLibrary.Conv_IntToString` _result)))))

(fn `UserConstructionScript`)