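; Base projectile actor, named as a parent, that flies straight ahead and removes itself.
; Tick moves it along the root component's forward vector by Velocity scaled by delta time, using a swept move.
; A Delay chained after the move in Tick destroys the actor about three seconds after its first tick.
; It implements no hit, overlap or damage logic.
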(event `self.ReceiveTick`
  (params (DeltaSeconds :type "Float (single-precision)"))
  (bind _defaultsceneroot (`self.DefaultSceneRoot`))
  (`self.K2_SetActorLocation` (+ (`SceneComponent.K2_GetComponentLocation` _defaultsceneroot) (* (`KismetMathLibrary.GetForwardVector` (`SceneComponent.K2_GetComponentRotation` _defaultsceneroot)) (* (`self.Velocity`) (`GameplayStatics.GetWorldDeltaSeconds`)))) true)
  (`KismetSystemLibrary.Delay` 3.0)
  (`self.K2_DestroyActor`))

(fn `UserConstructionScript`)