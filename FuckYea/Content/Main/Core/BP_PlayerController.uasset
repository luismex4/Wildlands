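; Player controller for placing turrets on the landscape in a toggleable build mode.
; Space toggles build mode and updates the main UI; Right cycles the selected construct and shows its name.
; Each tick a mouse trace moves the level's BP_BuildingSignal preview to the cursor, or parks it below ground outside build mode.
; Left click spawns the selection where the trace hits Landscape, unless the preview overlaps something.
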(event `self.ReceiveBeginPlay`
  (`self.InitializeUI`)
  (`self.InitializeVariables`))

(event `self.ReceiveTick`
  (params (DeltaSeconds :type "Float (single-precision)"))
  (`self.ShowBuildingSignal`))

(event `Key|LeftMouseButton`
  (params (Key :type "Key Structure" :default "AnyKey"))
  (:`Pressed`
    (if (and (`self.BuildMode`) (not (`/Game/Main/Blueprints/BP_BuildingSignal.IsOverlapping` (`self.BuildingSignal`))))
      (bind (_hitresult _hit_result) (`self.LineTraceMouse`))
      (if _hitresult
        (bind (_bblockinghit _binitialoverlap _time _location _impactpoint _normal _impactnormal _physmat _hitactor) (`GameplayStatics.BreakHitResult` _hit_result))
        (cast `Landscape` _hitactor)
        (`|SpawnActorFromClass` (`KismetArrayLibrary.Array_Get` (`self.AvailableConstructs`) (`self.SelectTurret`)) (`KismetMathLibrary.MakeTransform` _location) "Undefined" "OverrideRootScale")))))

(event `Key|Right`
  (params (Key :type "Key Structure" :default "AnyKey"))
  (:`Pressed`
    (bind _result (`/Engine/EditorBlueprintResources/StandardMacros.IncrementInt` (`self.SelectTurret`))
      (:`  `
        (if (>= _result (`KismetArrayLibrary.Array_Length` (`self.AvailableConstructs`)))
          (set `self.SelectTurret` 0))
        (`/Game/Main/Blueprints/UI/W_MainUI.SelectTurretSwitch` (`self.MainUI`) (`KismetSystemLibrary.GetClassDisplayName` (`KismetArrayLibrary.Array_Get` (`self.AvailableConstructs`) (`self.SelectTurret`))))))))

(event `Key|SpaceBar`
  (params (Key :type "Key Structure" :default "AnyKey"))
  (:`Pressed`
    (bind _output_get (set `self.BuildMode` (not (`self.BuildMode`))))
    (`/Game/Main/Blueprints/UI/W_MainUI.SetMode` (`self.MainUI`) (select `bool` _output_get :`false` "NewEnumerator0" :`true` "NewEnumerator1" :!type "/Game/Main/Data/E_GameMode Enum"))))

(fn `InitializeUI`
  (bind _returnvalue (`|CreateWidget` "/Game/Main/Blueprints/UI/W_MainUI.W_MainUI_C"))
  (bind _output_get (set `self.MainUI` _returnvalue))
  (`UserWidget.AddToViewport` _output_get 0))

(fn `InitializeVariables`
  (bind _outactors (`GameplayStatics.GetAllActorsOfClass` "/Game/Main/Blueprints/BP_BuildingSignal.BP_BuildingSignal_C"))
  (set `self.BuildingSignal` (`KismetArrayLibrary.Array_Get` _outactors)))

(fn `LineTraceMouse`
  (returns (HitResult :type Boolean) (`Hit Result` :type "HitResult Structure"))
  (bind (_worldlocation _worlddirection) (`self.DeprojectMousePositionToWorld`))
  (bind (_outhit _returnvalue) (`KismetSystemLibrary.LineTraceSingle` _worldlocation (+ _worldlocation (* _worlddirection 3000.0)) "TraceTypeQuery1" false (`|MakeArray` (`self.BuildingSignal`) :!type "Actor Object Reference") "None" true (struct :`R` 1.0 :`A` 1.0) (struct :`R` 1.0 :`A` 1.0)))
  (return _returnvalue _outhit))

(fn `ShowBuildingSignal`
  (if (`self.BuildMode`)
    (bind (_hitresult _hit_result) (`self.LineTraceMouse`))
    (`self.K2_SetActorLocation` (`self.BuildingSignal`) (`.Location` (`GameplayStatics.BreakHitResult` _hit_result)) false true)
    (else
      (`self.K2_SetActorLocation` (`self.BuildingSignal`) (0.0 0.0 -300.0) false true))))

(fn `UserConstructionScript`)